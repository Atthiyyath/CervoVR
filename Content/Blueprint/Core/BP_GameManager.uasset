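; Game manager for a wrap-around carousel of selectable objects that can be inspected one at a time.
; Changing the index teleports the chosen object and its two neighbours onto tagged TargetPoints.
; Interacting hides the neighbours and passes the object's name to it and BP_WidgetInfo; Back restores the neighbours and resets both.
; A Timeline with VInterpTo moves the player pawn toward tagged points, messaging "Pos2" once after finishing.
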(event `self.ReceiveBeginPlay`
  (set `self.TheRightOption` (- (`KismetArrayLibrary.Array_Length` (`self.Objects`)) 1))
  (set `self.TheLeftOption` 1))

(event `/Game/Blueprint/Interface/BPI_Interaction.SetActiveMainObject`
  (params (ID :type Integer))
  (bind _output_get (set `self.CurrentMultipleChoiceIndex` ID))
  (bind _currentmultiplechoiceindex (`self.SetCurrentChoice` _output_get))
  (`self.SetAfterChoice` _currentmultiplechoiceindex)
  (`self.SetBeforeChoice` _currentmultiplechoiceindex))

(event `/Game/Blueprint/Interface/BPI_Interaction.InteractWith`
  (params (ComponentName :type Name))
  (bind _objects (`self.Objects`))
  (bind _output (`|GetArrayItem` _objects (`self.TheRightOption`)))
  (bind _output_2 (`|GetArrayItem` _objects (`self.CurrentMultipleChoiceIndex`)))
  (bind _objectname (`/Game/Blueprint/BP_BaseObject.ObjectName` _output_2))
  (`/Engine/EditorBlueprintResources/StandardMacros.IsValid` _output
    (:`Is Valid`
      (`/Engine/EditorBlueprintResources/StandardMacros.IsValid` (`|GetArrayItem` _objects (`self.TheLeftOption`))
        (:`Is Valid`
          (`self.SetActorHiddenInGame` _output true)
          (`self.SetActorHiddenInGame` (`|GetArrayItem` _objects (`self.TheLeftOption`)) true))
        (:`Is Not Valid`
          _)))
    (:`Is Not Valid`
      _))
  (`self.SetActorHiddenInGame` _output_2 false)
  (`/Game/Blueprint/Interface/BPI_Interaction.RotateObject` _output_2 false)
  (`/Game/Blueprint/Interface/BPI_Interaction.InteractWith` _output_2 _objectname)
  (bind _outactors (`GameplayStatics.GetAllActorsOfClass` "/Game/Blueprint/Widget/BP_WidgetInfo.BP_WidgetInfo_C"))
  (`/Game/Blueprint/Interface/BPI_Interaction.InteractWith` (`|GetArrayItem` _outactors) _objectname))

(event `Back`
  (bind _objects (`self.Objects`))
  (bind _objects_2 (`self.Objects`))
  (bind _output (`|GetArrayItem` _objects_2 (`self.TheRightOption`)))
  (`/Engine/EditorBlueprintResources/StandardMacros.IsValid` _output
    (:`Is Valid`
      (`/Engine/EditorBlueprintResources/StandardMacros.IsValid` (`|GetArrayItem` _objects_2 (`self.TheLeftOption`))
        (:`Is Valid`
          (`self.SetActorHiddenInGame` _output false)
          (`self.SetActorHiddenInGame` (`|GetArrayItem` _objects_2 (`self.TheLeftOption`)) false))
        (:`Is Not Valid`
          _)))
    (:`Is Not Valid`
      _))
  (bind _outactors (`GameplayStatics.GetAllActorsOfClass` "/Game/Blueprint/Widget/BP_WidgetInfo.BP_WidgetInfo_C"))
  (`/Game/Blueprint/Interface/BPI_Interaction.InteractWith` (`|GetArrayItem` _outactors) "None")
  (`/Game/Blueprint/Interface/BPI_Interaction.InteractWith` (`|GetArrayItem` _objects (`self.CurrentMultipleChoiceIndex`)) "None")
  (for _array_element _objects
    (`/Engine/EditorBlueprintResources/StandardMacros.IsValid` _array_element
      (:`Is Valid`
        (`/Game/Blueprint/Interface/BPI_Interaction.RotateObject` _array_element true)))))

(event `/Game/Blueprint/Interface/BPI_Interaction.SetPositionPlayer`
  (params (TagPosition :type Name))
  (bind _returnvalue (`GameplayStatics.GetPlayerPawn` 0))
  (bind _outactors (`GameplayStatics.GetAllActorsOfClassWithTag` "/Script/Engine.TargetPoint" TagPosition))
  (bind _output (`|GetArrayItem` _outactors))
  (`/Engine/EditorBlueprintResources/StandardMacros.IsValid` _output
    (:`Is Valid`
      (bind (_direction _pos) (`Timeline|Timeline` :!via `PlayFromStart`)
        (:`Update`
          (`self.K2_SetActorLocation` _returnvalue (+ _pos (`KismetMathLibrary.VInterpTo` (`self.K2_GetActorLocation` _returnvalue) (`self.K2_GetActorLocation` _output) (`GameplayStatics.GetWorldDeltaSeconds`) 0.5)) false false))
        (:`Finished`
          (`/Engine/EditorBlueprintResources/StandardMacros.DoOnce` false
            (:`Completed`
              (message `/Game/Blueprint/Interface/BPI_Interaction.SetPositionPlayer` self "Pos2"))))))))

(fn `SetAfterChoice`
  (params (CurrentIndexOption :type Integer))
  (bind _objects (`self.Objects`))
  (bind _output (`|GetArrayItem` (`self.Objects`) (`self.TheRightOption`)))
  (bind _output_get (set `self.TheRightOption` CurrentIndexOption))
  (bind _result (`/Engine/EditorBlueprintResources/StandardMacros.IncrementInt` _output_get)
    (:`  `
      (if (< _result 0)
        (set `self.TheRightOption` (`KismetArrayLibrary.Array_LastIndex` _objects))
        (elif (> _result (- (`KismetArrayLibrary.Array_Length` _objects) 1))
          (set `self.TheRightOption` 0)))
      (bind _outactors (`GameplayStatics.GetAllActorsOfClassWithTag` "/Script/Engine.TargetPoint" "pos_3"))
      (`/Engine/EditorBlueprintResources/StandardMacros.IsValid` _output
        (:`Is Valid`
          (`self.K2_SetActorLocation` _output (`self.K2_GetActorLocation` (`|GetArrayItem` _outactors)) false false)
          (return))))))

(fn `SetBeforeChoice`
  (params (CurrentIndexOption :type Integer))
  (bind _objects (`self.Objects`))
  (bind _output (`|GetArrayItem` (`self.Objects`) (`self.TheLeftOption`)))
  (bind _output_get (set `self.TheLeftOption` CurrentIndexOption))
  (bind _result (`/Engine/EditorBlueprintResources/StandardMacros.DecrementInt` _output_get)
    (:`  `
      (if (< _result 0)
        (set `self.TheLeftOption` (`KismetArrayLibrary.Array_LastIndex` _objects))
        (elif (> _result (- (`KismetArrayLibrary.Array_Length` _objects) 1))
          (set `self.TheLeftOption` 0)))
      (bind _outactors (`GameplayStatics.GetAllActorsOfClassWithTag` "/Script/Engine.TargetPoint" "pos_2"))
      (`/Engine/EditorBlueprintResources/StandardMacros.IsValid` _output
        (:`Is Valid`
          (`self.K2_SetActorLocation` _output (`self.K2_GetActorLocation` (`|GetArrayItem` _outactors)) false false)
          (return))))))

(fn `SetCurrentChoice`
  (params (CurrentIndexOption :type Integer))
  (returns (CurrentMultipleChoiceIndex :type Integer))
  (bind _currentmultiplechoiceindex (`self.CurrentMultipleChoiceIndex`))
  (bind _objects (`self.Objects`))
  (bind _output (`|GetArrayItem` (`self.Objects`) _currentmultiplechoiceindex))
  (if (< CurrentIndexOption 0)
    (set `self.CurrentMultipleChoiceIndex` (`KismetArrayLibrary.Array_LastIndex` _objects))
    (elif (> CurrentIndexOption (- (`KismetArrayLibrary.Array_Length` _objects) 1))
      (set `self.CurrentMultipleChoiceIndex` 0)))
  (bind _outactors (`GameplayStatics.GetAllActorsOfClassWithTag` "/Script/Engine.TargetPoint" "pos_1"))
  (`/Engine/EditorBlueprintResources/StandardMacros.IsValid` _output
    (:`Is Valid`
      (`self.K2_SetActorLocation` _output (`self.K2_GetActorLocation` (`|GetArrayItem` _outactors)) false false)
      (return _currentmultiplechoiceindex))))

(fn `UserConstructionScript`)