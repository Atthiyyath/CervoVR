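; Base actor for a named object, apparently a motorcycle given its data table, with two child-actor icons (IconStang, IconBan).
; On BeginPlay it copies ObjectName into each icon's ParentName, and RotateObject sets the IsRotating flag.
; Tick, click and Interactwith do nothing; logic for spawning spare-part components from the data table, toggling their visibility and spinning yaw is left disconnected.
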(event `self.ReceiveBeginPlay`
  (bind _asbp_icon_comp (cast `/Game/Blueprint/Widget/BP_IconComp` (`ChildActorComponent.ChildActor` (`self.Icon_Stang`))))
  (set `/Game/Blueprint/Widget/BP_IconComp.ParentName` (`self.ObjectName`) _asbp_icon_comp)
  (bind _asbp_icon_comp_2 (cast `/Game/Blueprint/Widget/BP_IconComp` (`ChildActorComponent.ChildActor` (`self.Icon_Ban`))))
  (set `/Game/Blueprint/Widget/BP_IconComp.ParentName` (`self.ObjectName`) _asbp_icon_comp_2))

(event `self.ReceiveActorOnClicked`
  (params (ButtonPressed :type "Key Structure")))

(event `self.ReceiveTick`
  (params (DeltaSeconds :type "Float (single-precision)"))
  (if (`self.IsRotating`)
    _))

(event `/Game/Blueprint/Interface/BPI_Interaction.RotateObject`
  (params (IsRotating :type Boolean))
  (set `self.IsRotating` IsRotating))

(event `/Game/Blueprint/Interface/BPI_Interaction.InteractWith`
  (params (ComponentName :type Name)))

(fn `UserConstructionScript`)