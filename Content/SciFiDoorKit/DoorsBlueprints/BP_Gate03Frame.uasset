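; Sci-fi gate that opens and closes by trigger overlap and also drives a title and stage change in the level.
; Entering Door_trigger plays the open animation and hides the first BP_Title actor tagged "Title".
; Leaving waits through a delay, plays the close animation, then starts a timeline that moves the first "Stage" static mesh actor.
; Each update adds the timeline position to the current location, so movement accumulates.
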(event `self.Door_trigger.OnComponentBeginOverlap`
  (params (OverlappedComponent :type "PrimitiveComponent Object Reference") (OtherActor :type "Actor Object Reference") (OtherComp :type "PrimitiveComponent Object Reference") (OtherBodyIndex :type Integer) (bFromSweep :type Boolean) (SweepResult :type "HitResult Structure (by ref)"))
  (`SkeletalMeshComponent.PlayAnimation` (`self.SkeletalMesh`) "/Game/SciFiDoorKit/Meshes/Gate03/AS_Gate03AnimOpen.AS_Gate03AnimOpen" false)
  (bind _outactors (`GameplayStatics.GetAllActorsOfClassWithTag` "/Game/Blueprint/Widget/BP_Title.BP_Title_C" "Title"))
  (`self.SetActorHiddenInGame` (`|GetArrayItem` _outactors) true))

(event `self.Door_trigger.OnComponentEndOverlap`
  (params (OverlappedComponent :type "PrimitiveComponent Object Reference") (OtherActor :type "Actor Object Reference") (OtherComp :type "PrimitiveComponent Object Reference") (OtherBodyIndex :type Integer))
  (`KismetSystemLibrary.Delay` 5.0)
  (`SkeletalMeshComponent.PlayAnimation` (`self.SkeletalMesh`) "/Game/SciFiDoorKit/Meshes/Gate03/AS_Gate03AnimClose.AS_Gate03AnimClose" false)
  (bind _outactors (`GameplayStatics.GetAllActorsOfClassWithTag` "/Script/Engine.StaticMeshActor" "Stage"))
  (bind (_direction _pos) (`Timeline|Timeline` :!via `PlayFromStart`)
    (:`Update`
      (bind _output (`|GetArrayItem` _outactors))
      (`self.K2_SetActorLocation` _output (+ _pos (`self.K2_GetActorLocation` _output)) false false))))

(fn `UserConstructionScript`)